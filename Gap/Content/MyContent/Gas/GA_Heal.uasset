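; GA_Heal is a gameplay ability that casts a ground-targeted area heal on player characters, including the caster.
; It loops a targeting montage while a GAT_Decal target actor awaits user confirmation, then commits and plays the cast montage, both borrowed Stun montages.
; An Event.Combat.Target gameplay event triggers a debug-drawn sphere trace at the chosen location, sized by DecalSize, applying GE_Heal once per unique PlayerCharacter.
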(event Custom|LoopAnim
  (|PlayMontageandWaitProxy "None" "/Game/MyContent/Characters/Anims/AM_StunTarget.AM_StunTarget" 1.0 "None" true 1.0 0.0 false
    (:OnBlendOut
      (if (Variables|Default|GetIsTargeting)
        (CallFunction|LoopAnim)))
    (:OnInterrupted
      (if (Variables|Default|GetIsTargeting)
        (Ability|EndAbility)))))

(event Custom|CommitHeal
  (bind _returnvalue (Ability|CommitAbility))
  (if _returnvalue
    (|PlayMontageandWaitProxy "None" "/Game/MyContent/Characters/Anims/AM_StunCommit.AM_StunCommit" 1.0 "None" true 1.0 0.0 false
      (:then
        (Ability|Tasks|WaitGameplayEvent "(TagName=\"Event.Combat.Target\")" 0
          (:EventReceived
            (CallFunction|HealBeacon))))
      (:OnCompleted
        (Ability|EndAbility :!label _label))
      (:OnInterrupted
        (goto _label)))
    (else
      (Ability|EndAbility))))

(event Custom|HealBeacon
  (bind _location (Variables|Default|GetLocation))
  (bind _outhits (Collision|MultiSphereTraceForObjects _location _location (Variables|Default|GetDecal%20Size) (Utilities|Array|MakeArray "ObjectTypeQuery3") false 0 "ForDuration" false))
  (Utilities|Array|Clear (Variables|Default|GetHitEnemies))
  (for _array_element _outhits
    (bind _asplayer_character (Utilities|Casting|CastToPlayerCharacter (.HitActor (Collision|BreakHitResult _array_element))))
    (if (not (Utilities|Array|ContainsItem (Variables|Default|GetHitEnemies) _asplayer_character))
      (bind _asplayer_character_2 (Utilities|Casting|CastToPlayerCharacter (.HitActor (Collision|BreakHitResult _array_element))))
      (Utilities|Array|AddUnique (Variables|Default|GetHitEnemies) _asplayer_character_2)
      (Utilities|IsValid (Ability|GetAbilitySystemComponent (.HitActor (Collision|BreakHitResult _array_element)))
        (:Is%20Valid
          (GameplayEffects|ApplyGameplayEffectToSelf :self (Ability|GetAbilitySystemComponent (.HitActor (Collision|BreakHitResult _array_element))) :GameplayEffectClass "/Game/MyContent/Gas/GE_Heal.GE_Heal_C"))))))

(event Ability|EventActivateAbility
  (CallFunction|LoopAnim)
  (Variables|Default|SetIsTargeting true)
  (bind _data (|WaitTargetData :ConfirmationType "UserConfirmed" :Class "/Game/MyContent/Gas/GAT_Decal.GAT_Decal_C" :DecalSize (Variables|Default|GetDecal%20Size) :MaxRange 4e+02 :StartLocation (Class|GameplayAbility|MakeTargetLocationInfofromOwnerActor) :ReticleClass 0 :bDebug true)
    (:ValidData
      (Variables|Default|SetLocation (.Location (Collision|BreakHitResult (Ability|TargetData|GetHitResultfromTargetData _data))))
      (Variables|Default|SetIsTargeting false)
      (CallFunction|CommitHeal))))