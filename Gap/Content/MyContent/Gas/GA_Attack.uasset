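; GA_Attack is a Gameplay Ability that runs a looping melee attack combo.
; Each swing plays a montage section the owner supplies for the current combo counter.
; ComboStart and ComboEnd events open and close the window where another Attack event chains the next section; the counter resets when the ability ends.
; Hit events apply GE_Damage at the event's magnitude to living targets, sending a Damage event to those tagged HitReacting.
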(event Ability|EventActivateAbility
  (Ability|Tasks|WaitGameplayEvent "(TagName=\"Event.Combat.Attack\")" 0
    (:then
      (bind (_animmontage _sectionname _sectioncount) (Class|BPICombat|HandleHeavyAttackCombo(Message) (.OwnerActor (Utilities|Struct|BreakGameplayAbilityActorInfo (Ability|GetActorInfo))) (Math|Integer|%(Integer) (Variables|Default|GetComboCounter) (Variables|Default|GetComboCount)) :!label _label))
      (Variables|Default|SetComboCount _sectioncount)
      (|PlayMontageandWaitProxy "None" _animmontage 1.5 _sectionname false 1.0 0.0 false
        (:then
          (Utilities|ComboStart "(TagName=\"Event.Combat.ComboStart\")" false
            (:ExecOut
              (bind _payload (Ability|Tasks|WaitGameplayEvent "(TagName=\"Event.Combat.Hit\")" 0 true)
                (:then
                  (Development|PrintString (Utilities|String|Append "Combo sequence: " (Utilities|String|ToString(Integer) (Variables|Default|GetComboCounter))) true false "(R=0.039995,G=1.000000,B=0.214292,A=1.000000)" 1.0 "15"))
                (:EventReceived
                  (CallFunction|HandleHitEvent _payload true))))
            (:StartEvent
              (Utilities|ComboEnd "(TagName=\"Event.Combat.ComboEnd\")" false))))
        (:OnCompleted
          (Ability|EndAbility))))
    (:EventReceived
      (if (Variables|Default|GetCanAttack)
        (Variables|Default|SetCanAttack false)
        (goto _label)))))

(event Ability|EventOnEndAbility
  (params (bWasCancelled :type Boolean))
  (Variables|Default|SetCanAttack false)
  (Variables|Default|SetComboCounter 0))

(fn HandleHitEvent
  (params (EventPayload :type Gameplay%20Event%20Data%20Structure) (bDebug :type Boolean))
  (bind (_eventtag _instigator _target _optionalobject _optionalobject2 _contexthandle _instigatortags _targettags _eventmagnitude) (Utilities|Struct|BreakGameplayEventData EventPayload))
  (LocalVariables|SetInstigator _instigator)
  (LocalVariables|SetTarget _target)
  (LocalVariables|SetMagnitude _eventmagnitude)
  (if bDebug
    (Development|PrintString (Utilities|String|Append (Utilities|GetDisplayName (LocalVariables|GetInstigator)) " hit " (Utilities|GetDisplayName (LocalVariables|GetTarget)) " wtih magnitude: " (Utilities|String|ToString(Float) (LocalVariables|GetMagnitude))) true true "(R=1.000000,G=0.226708,B=0.160317,A=1.000000)"))
  (if (not (GameplayTags|HasMatchingGameplayTag (Ability|GetAbilitySystemComponent (LocalVariables|GetTarget)) "(TagName=\"Character.State.Death\")"))
    (GameplayEffects|ApplyGameplayEffectToSelf :self (Ability|GetAbilitySystemComponent (LocalVariables|GetTarget)) :GameplayEffectClass "/Game/MyContent/Gas/GE_Damage.GE_Damage_C" :Level (LocalVariables|GetMagnitude))
    (if (GameplayTags|HasMatchingGameplayTag (Ability|GetAbilitySystemComponent (LocalVariables|GetTarget)) "(TagName=\"Character.Combat.HitReacting\")")
      (Ability|SendGameplayEventtoActor (LocalVariables|GetTarget) "(TagName=\"Event.Combat.Damage\")"))))