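; BP_Enemy is an enemy character Blueprint that reacts to damage through the Gameplay Ability System.
; Health changes route to HandleDamage, where combat-tagged damage presses the Impact ability tag, or the Die tag at zero health while disabling capsule and mesh collision.
; Non-combat damage only prints a message, and Tick prints base health for debugging.
; GetHitReaction supplies hit montages, while HandleHeavyAttackCombo returns empty values.
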(event Custom|HealthChangeEvent
  (params (NewHealth :type Float%20%28single-precision%29) (EffectTags :type Gameplay%20Tag%20Container%20Structure))
  (CallFunction|HandleDamage EffectTags NewHealth))

(event EventBeginPlay
  (EventDispatchers|BindEventtoOnHealthChanged (delegate Custom|HealthChangeEvent)))

(event Collision|EventActorBeginOverlap
  (params (OtherActor :type Actor%20Object%20Reference)))

(event EventTick
  (params (DeltaSeconds :type Float%20%28single-precision%29))
  (bind _returnvalue (GameplayAttributes|GetAttributeSet (Variables|Default|GetAbilitySystemComponent) "/Script/Gap.GapAttributeSet"))
  (Development|PrintString (Utilities|String|Append "Enemy: " (Utilities|String|ToString(Float) (.basevalue (Variables|/Script/Gap.GapAttributeSet|GetHealth _returnvalue)))) true false "(R=0.000000,G=0.660000,B=1.000000,A=1.000000)" 0.0))

(fn ConstructionScript)

(fn HandleDamage
  (params (TagContainer :type Gameplay%20Tag%20Container%20Structure%20%28by%20ref%29) (InputPin :type Float%20%28double-precision%29))
  (bind _abilitysystemcomponent (Variables|Default|GetAbilitySystemComponent))
  ;[1 0.3133 0.9486] Check damage type by effect tag
  (if (GameplayTags|HasTag TagContainer "(TagName=\"Event.Combat.Damage\")")
    (if (!= InputPin 0.0)
      (Class|GapAbilitySystemComponent|AbilityInputTagPressed _abilitysystemcomponent "(TagName=\"Ability.Combat.Impact\")")
      (else
        (Class|GapAbilitySystemComponent|AbilityInputTagPressed _abilitysystemcomponent "(TagName=\"Ability.Main.Die\")")
        (Collision|SetCollisionEnabled (Variables|Default|GetCapsuleComponent) "NoCollision")
        (Collision|SetCollisionEnabled (Variables|Character|GetMesh) "NoCollision")))
    (else
      (Development|PrintString "Non combat damage"))))

(fn GetHitReaction
  (return (Variables|Default|GetAnim%20Montages)))

(fn HandleHeavyAttackCombo
  (params (Index :type Integer))
  (return 0 "None" 0))